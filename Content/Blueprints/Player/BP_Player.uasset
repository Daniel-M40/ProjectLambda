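; Player Blueprint that owns the HUD and pause menu widgets and handles pausing the game.
; BeginPlay creates both widgets, stores them and adds only the HUD to the viewport.
; Escape and P share one FlipFlop that alternates between showing the pause widget with the game paused and removing it with the game unpaused.
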(event EventBeginPlay
  (bind _returnvalue (UserInterface|CreateWidget "/Game/UI/BP_pauseWidget.BP_pauseWidget_C"))
  (Variables|Default|SetPauseWidget _returnvalue)
  (bind _returnvalue_2 (UserInterface|CreateWidget "/Game/UI/BP_HUD.BP_HUD_C"))
  (bind _output_get (Variables|Default|SetHUDWidget _returnvalue_2))
  (UserInterface|Viewport|AddtoViewport _output_get 0))

(event Input|KeyboardEvents|Escape
  (params (Key :type Key%20Structure :default "None"))
  (:Pressed
    (Utilities|FlowControl|FlipFlop
      (:A
        (UserInterface|Viewport|AddtoViewport (Variables|Default|GetPauseWidget) 0)
        (Game|SetGamePaused true))
      (:B
        (Widget|RemovefromParent (Variables|Default|GetPauseWidget))
        (Game|SetGamePaused false)))))

(event Input|KeyboardEvents|P
  (params (Key :type Key%20Structure :default "None"))
  (:Pressed
    (Utilities|FlowControl|FlipFlop
      (:A
        (UserInterface|Viewport|AddtoViewport (Variables|Default|GetPauseWidget) 0)
        (Game|SetGamePaused true))
      (:B
        (Widget|RemovefromParent (Variables|Default|GetPauseWidget))
        (Game|SetGamePaused false)))))

(fn ConstructionScript)