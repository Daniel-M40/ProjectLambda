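; Core game mode that sends the game to the game-over level when the player dies.
; On BeginPlay it caches player 0's pawn as a PlayerCharacter and, if the cast succeeds, shows the mouse cursor.
; Tick polls the cached player's IsAlive flag and opens GameOverLvl once it is false.
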(event EventBeginPlay
  (bind _asplayer_character (Utilities|Casting|CastToPlayerCharacter (Game|Player|GetPlayerPawn 0)))
  (Variables|Default|SetPlayer _asplayer_character)
  (Variables|/Script/Engine.PlayerController|SetbShowMouseCursor (Game|GetPlayerController 0) true))

(event EventTick
  (params (DeltaSeconds :type Float%20%28single-precision%29))
  (bind _player (Variables|Default|GetPlayer))
  (if (Utilities|IsValid _player)
    (if (not (Variables|/Script/ProjectLambda.PlayerCharacter|GetbIsAlive _player))
      (Game|OpenLevel(byName) (Variables|Default|GetGameOverLvl)))))

(fn ConstructionScript)